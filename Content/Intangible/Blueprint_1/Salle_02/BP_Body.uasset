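; BP_Body is an animated body actor with a looping, animated heart attached to its Spine2Socket.
; A looping 0.8-second timer nudges the MPC_Rainbow "Coords" parameter twice per cycle after short delays, giving a double-beat rhythm.
; A fast looping timer slowly yaws CampfireRoot and repeatedly sets Speed to 1.0 on the body's ABP_Mixamoded instance, if that cast succeeds.
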(event Custom|RotateAround
  (Transformation|AddActorLocalRotation (Variables|Default|GetCampfireRoot) (Math|Rotator|MakeRotator 0.0 0.0 0.025) false false)
  (CallFunction|SetAnimSpeed 1.0))

(event Custom|CustomEvent_0
  (Utilities|FlowControl|Delay 0.27)
  (bind _returnvalue (Rendering|Material|GetScalarParameterValue "/Game/Intangible/Geometry_1/Materials/Salle_02/Materials/MPC_Rainbow.MPC_Rainbow" "Coords" :!class /Script/Engine.KismetMaterialLibrary))
  (Rendering|Material|SetScalarParameterValue "/Game/Intangible/Geometry_1/Materials/Salle_02/Materials/MPC_Rainbow.MPC_Rainbow" "Coords" (+ _returnvalue 0.05) :!class /Script/Engine.KismetMaterialLibrary)
  (Utilities|FlowControl|Delay 0.2)
  (bind _returnvalue_2 (Rendering|Material|GetScalarParameterValue "/Game/Intangible/Geometry_1/Materials/Salle_02/Materials/MPC_Rainbow.MPC_Rainbow" "Coords" :!class /Script/Engine.KismetMaterialLibrary))
  (Rendering|Material|SetScalarParameterValue "/Game/Intangible/Geometry_1/Materials/Salle_02/Materials/MPC_Rainbow.MPC_Rainbow" "Coords" (+ _returnvalue_2 0.05) :!class /Script/Engine.KismetMaterialLibrary))

(event EventBeginPlay
  (Transformation|AttachComponentToComponent (Variables|Default|GetHeart) (Variables|Default|GetBody) "Spine2Socket" "KeepWorld" "KeepWorld" "KeepRelative" true)
  (Components|Animation|PlayAnimation (Variables|Default|GetHeart) "/Game/Intangible/Geometry_1/Meshes/Salle_02/Coeur/coeur_animated_Anim.coeur_animated_Anim" true)
  (Components|Animation|PlayAnimation (Variables|Default|GetBody) "/Game/Intangible/Geometry_1/Meshes/Salle_02/Body/body_mixamod_Anim.body_mixamod_Anim" true)
  (Utilities|Time|SetTimerbyEvent (delegate Custom|CustomEvent_0) 0.8 true)
  (Utilities|Time|SetTimerbyEvent (delegate Custom|RotateAround) 0.01 true))

(event Collision|EventActorBeginOverlap
  (params (OtherActor :type Actor%20Object%20Reference)))

(event EventTick
  (params (DeltaSeconds :type Float%20%28single-precision%29)))

(fn ConstructionScript)

(fn SetAnimSpeed
  (params (Speed :type Float%20%28single-precision%29))
  (bind _asabp_mixamoded (Utilities|Casting|CastToABP_Mixamoded (Components|SkeletalMesh|GetAnimInstance (Variables|Default|GetBody))))
  (Variables|/Game/Intangible/Geometry_1/Meshes/Salle_02/Body/ABP_Mixamoded.ABP_Mixamoded_C|SetSpeed _asabp_mixamoded Speed))