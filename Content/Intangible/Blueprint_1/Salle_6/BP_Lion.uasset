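; BP_Lion is a lion artwork in Salle_6 that endlessly alternates between its normal look and a sequined, glitched one.
; From BeginPlay, a FlipFlop swaps the static mesh and stores the matching material, which a second event applies to slot 0.
; That event restarts the cycle after five seconds.
; On the glitched pass, a two-second delay makes the material change lag behind the mesh swap.
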(event Custom|Switch_Mesh
  (Utilities|FlowControl|FlipFlop
    (:A
      (Components|StaticMesh|SetStaticMesh (Variables|Default|GetOeuvre) (Variables|Default|GetLion_Normale))
      (Variables|Default|SetM_Oeuvre (Variables|Default|GetM_Normale)))
    (:B
      (Components|StaticMesh|SetStaticMesh (Variables|Default|GetOeuvre) (Variables|Default|GetLion_Pailette))
      (Variables|Default|SetM_Oeuvre (Variables|Default|GetM_Glitched))
      (Utilities|FlowControl|Delay 2.0)))
  (CallFunction|SwitchMaterial))

(event Custom|Switch_Material
  (Rendering|Material|SetMaterial (Variables|Default|GetOeuvre) 0 (Variables|Default|GetM_Oeuvre))
  (Utilities|FlowControl|Delay 5.0)
  (CallFunction|SwitchMesh))

(event EventBeginPlay
  (CallFunction|SwitchMesh))

(fn ConstructionScript)