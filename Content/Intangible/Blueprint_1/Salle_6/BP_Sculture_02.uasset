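; BP_Sculture_02 is a sculpture actor in Salle_6 that tumbles and flickers between mesh levels of detail.
; A timeline started on BeginPlay drives roll and pitch together from 0 to 360 degrees, feeding in the static mesh's current yaw.
; A looping timer, with its short interval randomized once at start, forces a random LOD on the mesh, using LOD switching as a visual glitch effect.
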(event Custom|LOD
  (Rendering|LOD|SetForcedLodModel (Variables|Default|GetStaticMesh) (Math|Random|RandomIntegerinRange 0 8)))

(event EventBeginPlay
  (Utilities|Time|SetTimerbyEvent (delegate Custom|LOD) (Math|Random|RandomFloatinRange 0.1 0.2) true)
  (bind _newtrack_0 (Timeline|Timeline_0 PlayFromStart)
    (:Update
      (Transformation|SetActorRotation (Math|Rotator|MakeRotator (Math|Float|Lerp 0.0 3.6e+02 _newtrack_0) (Math|Float|Lerp 0.0 3.6e+02 _newtrack_0) (.yaw (Transformation|GetWorldRotation (Variables|Default|GetStaticMesh))))))))

(fn ConstructionScript)