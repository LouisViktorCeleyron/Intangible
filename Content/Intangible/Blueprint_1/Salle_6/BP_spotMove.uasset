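; BP_spotMove animates a moving spotlight, apparently for room 6 (Salle 6), spinning it while swinging it back and forth.
; Tick runs through a short Delay, so each step adds a constant local rotation on one axis at a throttled rate.
; A counter and the StartClosed flag alternate equal runs of positive and negative steps on a second axis, then reset to loop the swing.
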(event EventTick
  (params (DeltaSeconds :type Float%20%28single-precision%29))
  (Utilities|FlowControl|Delay 0.05)
  (Transformation|AddLocalRotation (Variables|Default|GetSpotLightComponent) "3.000000,0.000000, 0" false false)
  (if (< (Variables|Default|GetCount) 20)
    (Variables|Default|SetStart%20Closed true)
    (Transformation|AddLocalRotation (Variables|Default|GetSpotLightComponent) "0,3.000000, 0" false false)
    (Variables|Default|SetCount (+ (Variables|Default|GetCount) 1))
    (else
      (Utilities|FlowControl|Sequence
        (:then_0
          (if (Variables|Default|GetStart%20Closed)
            (Variables|Default|SetCount 40)
            (Variables|Default|SetStart%20Closed false)))
        (:then_1
          (Transformation|AddLocalRotation (Variables|Default|GetSpotLightComponent) "0,-3.000000, 0" false false)
          (bind _output_get (Variables|Default|SetCount (+ (Variables|Default|GetCount) -1)))
          (if (== _output_get 20)
            (Variables|Default|SetCount 0)))))))

(fn ConstructionScript)