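; BP_Spline_Air is an emitter actor in Salle_8 that periodically spawns BP_Objet_Spline_Air objects at its own transform.
; Tick decrements a Delay counter and, at zero, resets it and spawns a new object, so the spawn rate depends on frame rate.
; Each spawned object receives this actor through InitializeAir, linking it back to its emitter.
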(event EventBeginPlay)

(event Collision|EventActorBeginOverlap
  (params (OtherActor :type Actor%20Object%20Reference)))

(event EventTick
  (params (DeltaSeconds :type Float%20%28single-precision%29))
  (if (== 0 (Variables|Default|GetDelay))
    (Variables|Default|SetDelay 100)
    (bind _returnvalue (Game|SpawnActorfromClass "/Game/Intangible/Blueprint_1/Salle_8/BP_Objet_Spline_Air.BP_Objet_Spline_Air_C" (Transformation|GetActorTransform) "Undefined" 0 0))
    (Default|InitializeAir _returnvalue self)
    (else
      (Variables|Default|SetDelay (- (Variables|Default|GetDelay) 1)))))

(fn ConstructionScript)