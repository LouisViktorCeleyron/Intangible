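; BP_Objet_Spline is an actor that travels once along a spline from start to end, then destroys itself.
; On BeginPlay it finds a BP_Spline in the level and starts a timeline with play rate set to 1/Time.
; Each update lerps the timeline value over the spline length, taking location in world space but rotation in local space.
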(event Custom|Move%20Object
  (bind _ref_spline (Variables|Default|GetREF%20Spline))
  (bind _spline (Variables|/Game/Intangible/Blueprint_1/Salle_8/BP_Spline.BP_Spline_C|GetSpline _ref_spline))
  (Components|Timeline|SetPlayRate (Variables|Default|GetTimeline_0) (/ 1.0 (Variables|Default|GetTime)))
  (bind _newtrack_0 (Timeline|Timeline_0 Play)
    (:Update
      (Transformation|SetActorTransform (Math|Transform|MakeTransform (Spline|GetLocationatDistanceAlongSpline _spline (Math|Float|Lerp 0.0 (Spline|GetSplineLength (Variables|/Game/Intangible/Blueprint_1/Salle_8/BP_Spline.BP_Spline_C|GetSpline (Variables|Default|GetREF%20Spline))) _newtrack_0) "World") (Spline|GetRotationatDistanceAlongSpline _spline (Math|Float|Lerp 0.0 (Spline|GetSplineLength (Variables|/Game/Intangible/Blueprint_1/Salle_8/BP_Spline.BP_Spline_C|GetSpline (Variables|Default|GetREF%20Spline))) _newtrack_0) "Local") "1,1,1")))
    (:Finished
      (Actor|DestroyActor))))

(event EventBeginPlay
  (bind _returnvalue (Actor|GetActorOfClass "/Game/Intangible/Blueprint_1/Salle_8/BP_Spline.BP_Spline_C"))
  (Variables|Default|SetREF%20Spline _returnvalue)
  (CallFunction|MoveObject))

(fn ConstructionScript)