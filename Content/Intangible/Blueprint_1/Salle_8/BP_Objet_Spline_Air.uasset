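; BP_Objet_Spline_Air is an actor that travels once along an air spline and then destroys itself.
; On BeginPlay it gives its Cube a random mesh from ListMesh.
; Initialize_air receives the spline reference and starts MoveObjectAir, where a timeline with play rate scaled by Time drives distance along the spline.
; Each update sets location in world space but takes rotation in the spline's local space.
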(event Custom|Move%20Object%20air
  (bind _ref_spline (Variables|Default|GetREF%20Spline))
  (bind _spline_air (Variables|/Game/Intangible/Blueprint_1/Salle_8/BP_Spline_Air.BP_Spline_Air_C|GetSpline_air _ref_spline))
  (Components|Timeline|SetPlayRate (Variables|Default|GetTimeline_0) (/ 1.0 (Variables|Default|GetTime)))
  (bind _newtrack_0 (Timeline|Timeline_0 Play)
    (:Update
      (Transformation|SetActorTransform (Math|Transform|MakeTransform (Spline|GetLocationatDistanceAlongSpline _spline_air (Math|Float|Lerp 0.0 (Spline|GetSplineLength (Variables|/Game/Intangible/Blueprint_1/Salle_8/BP_Spline_Air.BP_Spline_Air_C|GetSpline_air (Variables|Default|GetREF%20Spline))) _newtrack_0) "World") (Spline|GetRotationatDistanceAlongSpline _spline_air (Math|Float|Lerp 0.0 (Spline|GetSplineLength (Variables|/Game/Intangible/Blueprint_1/Salle_8/BP_Spline_Air.BP_Spline_Air_C|GetSpline_air (Variables|Default|GetREF%20Spline))) _newtrack_0) "Local") "1,1,1")))
    (:Finished
      (Actor|DestroyActor))))

(event Custom|Initialize_air
  (params (REF%20Spline :type BP%20Spline%20Air%20Object%20Reference))
  (Variables|Default|SetREF%20Spline REF%20Spline)
  (CallFunction|MoveObjectAir))

(event EventBeginPlay
  (Components|StaticMesh|SetStaticMesh (Variables|Default|GetCube) (.OutItem (Utilities|Array|Random (Variables|Default|GetList%20mesh)))))

(fn ConstructionScript)