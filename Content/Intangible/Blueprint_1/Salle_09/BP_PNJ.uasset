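; NPC actor for Salle_09 that repeatedly appears, walks along a set path and resets.
; A looping timer ramps the "Appearance" scalar in MPC_Body until full, then starts the walk animation and a timeline.
; The timeline moves the root along negative X and drives its height from a second track.
; On finish it zeroes the shared parameter, returns to the start and stops the animation, restarting the cycle.
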(event Custom|Appearance
  (bind _defaultsceneroot (Variables|Default|GetDefaultSceneRoot))
  (bind _defaultsceneroot_2 (Variables|Default|GetDefaultSceneRoot))
  (bind _basepos (Variables|Default|GetBasePos))
  (bind _returnvalue (Transformation|GetWorldLocation _defaultsceneroot_2))
  (bind _x (Math|Vector|BreakVector _basepos))
  (bind _returnvalue_2 (Transformation|GetWorldLocation _defaultsceneroot))
  (bind _returnvalue_3 (Rendering|Material|GetScalarParameterValue "/Game/Intangible/Geometry_1/Materials/Salle_9/MPC_Body.MPC_Body" "Appearance" :!class /Script/Engine.KismetMaterialLibrary))
  (if (>= _returnvalue_3 1.0)
    (if (not (Variables|Default|Getappeared))
      (Variables|Default|Setappeared true)
      (Components|Animation|PlayAnimation (Variables|Default|GetBodyPNJ) "/Game/Intangible/Geometry_1/Meshes/Salle_9/Anime/Walking_Anim.Walking_Anim" true)
      (bind (_direction _newtrack_0 _movedwn) (Timeline|Timeline_0 PlayFromStart)
        (:Update
          (Transformation|SetWorldLocation (Variables|Default|GetDefaultSceneRoot) (Math|Vector|MakeVector (Math|Float|Lerp _x (+ _x -5e+03) _newtrack_0) (.y _returnvalue_2) (.z _returnvalue_2)) false false)
          (Transformation|SetWorldLocation (Variables|Default|GetDefaultSceneRoot) (Math|Vector|MakeVector (.x _returnvalue) (.y _returnvalue) _movedwn) false false))
        (:Finished
          (Rendering|Material|SetScalarParameterValue "/Game/Intangible/Geometry_1/Materials/Salle_9/MPC_Body.MPC_Body" "Appearance" 0.0 :!class /Script/Engine.KismetMaterialLibrary)
          (Variables|Default|Setappeared false)
          (Transformation|SetWorldLocation (Variables|Default|GetDefaultSceneRoot) (Variables|Default|GetBasePos) false false)
          (Components|Animation|SetPosition (Variables|Default|GetBodyPNJ) 0.0 true)
          (Audio|Components|Audio|Stop (Variables|Default|GetBodyPNJ)))))
    (else
      (bind _returnvalue_4 (Rendering|Material|GetScalarParameterValue "/Game/Intangible/Geometry_1/Materials/Salle_9/MPC_Body.MPC_Body" "Appearance" :!class /Script/Engine.KismetMaterialLibrary))
      (Rendering|Material|SetScalarParameterValue "/Game/Intangible/Geometry_1/Materials/Salle_9/MPC_Body.MPC_Body" "Appearance" (+ _returnvalue_4 0.01) :!class /Script/Engine.KismetMaterialLibrary))))

(event EventBeginPlay
  (Variables|Default|SetBasePos (Transformation|GetActorLocation))
  (Utilities|Time|SetTimerbyEvent (delegate Custom|Appearance) 0.1 true))

(event Collision|EventActorBeginOverlap
  (params (OtherActor :type Actor%20Object%20Reference)))

(event EventTick
  (params (DeltaSeconds :type Float%20%28single-precision%29)))

(fn ConstructionScript)