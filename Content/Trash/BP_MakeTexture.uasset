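; BP_MakeTexture is an actor that paints a trail of its own position into a render target fed to a landscape material.
; BeginPlay passes MyRenderTarget to the landscape's RenderTarget parameter, clears it to black and creates an unused M_LandscapeTest dynamic instance.
; Each Tick remaps actor XY from a fixed world range to normalized coordinates and stamps T_Painting there via canvas drawing, accumulating without further clears.
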(event EventBeginPlay
  (Rendering|Material|CreateDynamicMaterialInstance "/Game/Trash/M_LandscapeTest.M_LandscapeTest" "None" "None" :!class /Script/Engine.KismetMaterialLibrary)
  (Landscape|Runtime|Material|SetLandscapeMaterialTextureParameterValue (Variables|Default|GetLandscape) "RenderTarget" "/Game/Trash/MyRenderTarget.MyRenderTarget")
  (Rendering|ClearRenderTarget2D "/Game/Trash/MyRenderTarget.MyRenderTarget"))

(event Collision|EventActorBeginOverlap
  (params (OtherActor :type Actor%20Object%20Reference)))

(event EventTick
  (params (DeltaSeconds :type Float%20%28single-precision%29))
  (bind _returnvalue (Transformation|GetActorLocation))
  (bind _returnvalue_2 (/ _returnvalue 1.4e+03))
  (bind _returnvalue_3 (+ _returnvalue_2 1.0))
  (bind _returnvalue_4 (/ _returnvalue_3 2.0))
  (bind (_x _y) (Math|Vector|BreakVector _returnvalue_4))
  (CallFunction|DrawPlayerPositiononCanevas (Math|Vector2D|MakeVector2D _x _y) 1e+01))

(fn ConstructionScript)

(fn DrawPlayerPositiononCanevas
  (params (Location :type Vector%202D%20Structure) (Size :type Float%20%28single-precision%29))
  (bind (_canvas _size _context) (Rendering|BeginDrawCanvastoRenderTarget "/Game/Trash/MyRenderTarget.MyRenderTarget"))
  (Canvas|DrawTexture :self _canvas :RenderTexture "/Game/Trash/T_Painting.T_Painting" :ScreenPosition (* _size Location) :ScreenSize (Math|Vector2D|MakeVector2D Size Size) :CoordinateSize "(X=1.000000,Y=1.000000)" :PivotPoint "(X=0.500000,Y=0.500000)")
  (Rendering|EndDrawCanvastoRenderTarget _context))