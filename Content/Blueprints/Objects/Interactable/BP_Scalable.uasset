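; BP_Scalable is a randomly colored VR interactable sphere that players resize by changing the distance between their hands.
; Box overlap subscribes it to the pawn's interaction component; untriggered interaction tracks hand distance, and triggered interaction applies the change through AddScale, also adjusting a material scalar.
; At a size threshold it locks input and plays the LooseControl timeline, which keeps growing it, then spawns and subscribes a fresh copy.
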(event OnComponentBeginOverlap(Box)
  (params (OverlappedComponent :type Primitive%20Component%20Object%20Reference) (OtherActor :type Actor%20Object%20Reference) (OtherComp :type Primitive%20Component%20Object%20Reference) (OtherBodyIndex :type Integer) (bFromSweep :type Boolean) (SweepResult :type Hit%20Result%20Structure%20%28by%20ref%29))
  (bind _asbp_vrplayer_pawn (Utilities|Casting|CastToBP_VRPlayerPawn OtherActor))
  (Variables|Default|SetBP%20AC%20Interract%20with%20Interactable (Variables|/Game/Blueprints/Pawn/BP_VRPlayerPawn.BP_VRPlayerPawn_C|GetBP_AC_InterractWithInteractable _asbp_vrplayer_pawn))
  (Variables|/Game/Blueprints/Component/ActorComponent/BP_AC_InterractWithInteractable.BP_AC_InterractWithInteractable_C|SetInterractableSubscribed (Variables|/Game/Blueprints/Pawn/BP_VRPlayerPawn.BP_VRPlayerPawn_C|GetBP_AC_InterractWithInteractable _asbp_vrplayer_pawn) self))

(event EventInteractButNotTrigger
  (params (Player :type BP%20VR%20Player%20Pawn%20Object%20Reference))
  (if (not (Variables|Default|GetStop))
    (Variables|Default|SetTempDistance (Math|Vector|Distance(Vector) (Transformation|GetWorldLocation (Variables|/Game/Blueprints/Pawn/BP_VRPlayerPawn.BP_VRPlayerPawn_C|GetRight Player)) (Transformation|GetWorldLocation (Variables|/Game/Blueprints/Pawn/BP_VRPlayerPawn.BP_VRPlayerPawn_C|GetLeft Player))))))

(event EventBeginPlay
  (bind _sphere (Variables|Default|GetSphere))
  (bind _returnvalue (Rendering|Material|CreateDynamicMaterialInstance _sphere 0 (Rendering|Material|GetMaterial _sphere 0) "None" :!class /Script/Engine.PrimitiveComponent))
  (bind _output_get (Variables|Default|SetMaterial _returnvalue))
  (Rendering|Material|SetVectorParameterValue _output_get "Param" (Math|Color|MakeColor (Math|Random|RandomFloat) (Math|Random|RandomFloat) (Math|Random|RandomFloat)) :!class /Script/Engine.MaterialInstanceDynamic))

(event EventInteractandTrigger
  (params (Player :type BP%20VR%20Player%20Pawn%20Object%20Reference))
  (bind _loosecontrol (Variables|Default|GetLooseControl))
  (bind _right (Variables|/Game/Blueprints/Pawn/BP_VRPlayerPawn.BP_VRPlayerPawn_C|GetRight Player))
  (bind _left (Variables|/Game/Blueprints/Pawn/BP_VRPlayerPawn.BP_VRPlayerPawn_C|GetLeft Player))
  (bind _returnvalue (Transformation|GetWorldLocation _right))
  (bind _returnvalue_2 (Transformation|GetWorldLocation _left))
  (bind _returnvalue_3 (Math|Vector|Distance(Vector) _returnvalue _returnvalue_2))
  (if (not (Variables|Default|GetStop))
    (CallFunction|AddScale (* 0.1 (- _returnvalue_3 (Variables|Default|GetTempDistance))))
    (Variables|Default|SetTempDistance _returnvalue_3)
    (if (>= (Variables|Default|GetScaleFactor) (Variables|Default|GetScaleBeforeEvent))
      (Variables|Default|SetStop true)
      (Components|Timeline|SetPlayRate _loosecontrol 0.1)
      (Components|Timeline|PlayfromStart _loosecontrol))))

(fn ConstructionScript)

(fn AddScale
  (params (Delta :type Float%20%28single-precision%29))
  (bind _material (Variables|Default|GetMaterial))
  (bind _output_get (Variables|Default|SetScaleFactor (Math|Float|Clamp(Float) (+ (Variables|Default|GetScaleFactor) Delta) 1.0 1e+02)))
  (Transformation|SetWorldScale3D (Variables|Default|GetSphere) (* (Class|KismetMathLibrary|VectorOne) _output_get))
  (bind _returnvalue (Rendering|Material|GetScalarParameterValue _material "Param" :!class /Script/Engine.MaterialInstanceDynamic))
  (Rendering|Material|SetScalarParameterValue _material "Param" (+ _returnvalue Delta) :!class /Script/Engine.MaterialInstanceDynamic))