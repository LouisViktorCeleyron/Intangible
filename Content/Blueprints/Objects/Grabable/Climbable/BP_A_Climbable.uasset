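; Climbable actor that turns a motion controller grab into a climb action on the player pawn.
; When GrabComponent fires OnGrabbed, it matches the controller to the pawn's Left or Right one and calls ClimbEvent with the corresponding hand enum.
; Dropping triggers no logic here, and the PlayerPawn reference cached at BeginPlay is not used by the grab handler.
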(event OnGrabbed(GrabComponent)
  (params (MotionController :type Motion%20Controller%20Component%20Object%20Reference))
  (bind _playerpawn (CallFunction|GetMyPawn))
  (bind _playerpawn_2 (CallFunction|GetMyPawn))
  (Utilities|FlowControl|Sequence
    (:then_0
      (if (== MotionController (Variables|/Game/Blueprints/Pawn/BP_VRPlayerPawn.BP_VRPlayerPawn_C|GetLeft _playerpawn_2))
        (Default|ClimbEvent _playerpawn_2 "NewEnumerator0")))
    (:then_1
      (if (== MotionController (Variables|/Game/Blueprints/Pawn/BP_VRPlayerPawn.BP_VRPlayerPawn_C|GetRight _playerpawn))
        (Default|ClimbEvent _playerpawn "NewEnumerator1")))))

(event OnDropped(GrabComponent))

(event EventBeginPlay
  (|CallParentFunction)
  (Variables|Default|SetPlayerPawn (CallFunction|GetMyPawn)))

(event Collision|EventActorBeginOverlap
  (params (OtherActor :type Actor%20Object%20Reference))
  (|CallParentFunction OtherActor) ; This node is disabled and will not be called.\nDrag off pins to build functionality.
)

(event EventTick
  (params (DeltaSeconds :type Float%20%28single-precision%29))
  (|CallParentFunction DeltaSeconds) ; This node is disabled and will not be called.\nDrag off pins to build functionality.
)

(fn ConstructionScript
  (|CallParentFunction))