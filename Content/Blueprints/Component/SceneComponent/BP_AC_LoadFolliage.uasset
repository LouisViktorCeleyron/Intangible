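; BP_AC_LoadFolliage is a scene component that triggers growth on nearby NewBlueprint actors, apparently foliage, around its world location.
; Every Tick it runs a sphere overlap of the given Radius on WorldStatic objects, filtered to NewBlueprint, and calls Grow on each result.
; Grow is called again each frame while an actor stays in range, as the component tracks no state.
; A Debug flag draws the search sphere.
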(event EventBeginPlay)

(event EventTick
  (params (DeltaSeconds :type Float%20%28single-precision%29))
  (Utilities|FlowControl|Sequence
    (:then_0
      (if (Variables|Default|Getdebug)
        (Rendering|Debug|DrawDebugSphere (Transformation|GetWorldLocation) (Variables|Default|GetRadius) 12 "(R=1.000000,G=1.000000,B=1.000000,A=1.000000)" 0.0)))
    (:then_1
      (bind _outactors (Collision|SphereOverlapActors (Transformation|GetWorldLocation) (Variables|Default|GetRadius) (Utilities|Array|MakeArray "ObjectTypeQuery1") "/Game/Trash/NewBlueprint.NewBlueprint_C"))
      (for _array_element _outactors
        (bind _asnew_blueprint (Utilities|Casting|CastToNewBlueprint _array_element))
        (Default|Grow _asnew_blueprint)))))