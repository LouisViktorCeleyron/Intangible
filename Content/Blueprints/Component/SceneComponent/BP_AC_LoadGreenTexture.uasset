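; Scene component that paints its world position into a render target used by the Landscape material, leaving a trail as it moves.
; On BeginPlay it binds the target to the material's RenderTarget parameter and clears it to black.
; Each Tick maps world XY to UVs over a fixed, origin-centered area and stamps a Radius-sized brush texture there.
; The target is never cleared during play, so stamps accumulate.
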(event EventBeginPlay
  (bind _returnvalue (Actor|GetActorOfClass "/Script/Landscape.Landscape"))
  (Landscape|Runtime|Material|SetLandscapeMaterialTextureParameterValue _returnvalue "RenderTarget" "/Game/Trash/MyRenderTarget.MyRenderTarget")
  (Rendering|ClearRenderTarget2D "/Game/Trash/MyRenderTarget.MyRenderTarget"))

(event EventTick
  (params (DeltaSeconds :type Float%20%28single-precision%29))
  (bind _returnvalue (Transformation|GetWorldLocation))
  (bind _returnvalue_2 (/ _returnvalue 1.4e+03))
  (bind _returnvalue_3 (+ _returnvalue_2 1.0))
  (bind _returnvalue_4 (/ _returnvalue_3 2.0))
  (bind (_x _y) (Math|Vector|BreakVector _returnvalue_4))
  (CallFunction|DrawPositiononTexture (Math|Vector2D|MakeVector2D _x _y)))

(fn DrawPositiononTexture
  (params (Location :type Vector%202D%20Structure))
  (bind _radius (Variables|Default|GetRadius))
  (bind (_canvas _size _context) (Rendering|BeginDrawCanvastoRenderTarget "/Game/Trash/MyRenderTarget.MyRenderTarget"))
  (Canvas|DrawTexture :self _canvas :RenderTexture "/Game/Trash/T_Painting.T_Painting" :ScreenPosition (- (* _size Location) (/ (Variables|Default|GetRadius) 2.0)) :ScreenSize (Math|Vector2D|MakeVector2D _radius _radius) :CoordinateSize "(X=1.000000,Y=1.000000)" :PivotPoint "(X=0.500000,Y=0.500000)")
  (Rendering|EndDrawCanvastoRenderTarget _context))