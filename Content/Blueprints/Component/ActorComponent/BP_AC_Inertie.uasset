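; Actor component for BP_VRPlayerPawn that computes inertia and gravity displacement for the VR player.
; Each tick it derives a per-frame velocity from the root's position change since the last frame, Verlet-style.
; It adds gravity scaled by delta time squared only while neither left nor right is held.
; The resulting Displacement is only stored, as the SetActorLocation call is disconnected.
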(event EventBeginPlay
  (bind _asbp_vrplayer_pawn (Utilities|Casting|CastToBP_VRPlayerPawn (Components|GetOwner)))
  (bind _output_get (Variables|Default|SetVRPlayer _asbp_vrplayer_pawn))
  (Variables|Default|SetlastPosition (Transformation|GetWorldLocation (Variables|/Game/Blueprints/Pawn/BP_VRPlayerPawn.BP_VRPlayerPawn_C|GetDefaultSceneRoot _output_get))))

(event EventTick
  (params (DeltaSeconds :type Float%20%28single-precision%29))
  (bind _returnvalue (Utilities|Time|GetWorldDeltaSeconds))
  (bind _vrplayer (Variables|Default|GetVRPlayer))
  (bind _vrplayer_2 (Variables|Default|GetVRPlayer))
  (bind _rootcomponent (Variables|/Script/Engine.Actor|GetRootComponent _vrplayer_2))
  (bind _returnvalue_2 (Transformation|GetWorldLocation _rootcomponent))
  (Utilities|FlowControl|Sequence
    (:then_0
      (Variables|Default|SetIsAffectedByGravity (not (or (Variables|/Game/Blueprints/Pawn/BP_VRPlayerPawn.BP_VRPlayerPawn_C|GetLeftIsHeld _vrplayer) (Variables|/Game/Blueprints/Pawn/BP_VRPlayerPawn.BP_VRPlayerPawn_C|GetRightIsHeld _vrplayer)))))
    (:then_1
      (Variables|Default|SetcurrentVelocity (- _returnvalue_2 (Variables|Default|GetlastPosition))))
    (:then_2
      (Variables|Default|SetDisplacement (+ "0, 0, 0" (* (Variables|Default|GetcurrentVelocity) 1.0) (* (* (* (Variables|Default|GetcurrentGravity) (select (Variables|Default|GetIsAffectedByGravity) 1.0 0.0)) _returnvalue) _returnvalue))))
    (:then_3
      (Variables|Default|SetlastPosition _returnvalue_2))))