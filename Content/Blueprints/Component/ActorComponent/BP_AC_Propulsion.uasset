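; BP_AC_Propulsion is an actor component that computes a hand-directed boost vector for the VR player pawn.
; On BeginPlay it caches the owning BP_VRPlayerPawn, its left and right particle systems, and the capsule's starting location.
; Each Tick sums both hands' forward vectors, scaled by BoostPower and delta time while either boost input is active, otherwise zero.
; The result is only stored in Boost; this graph neither moves the pawn nor drives the particles.
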(event EventBeginPlay
  (bind _asbp_vrplayer_pawn (Utilities|Casting|CastToBP_VRPlayerPawn (Components|GetOwner)))
  (bind _output_get (Variables|Default|SetVRPlayer _asbp_vrplayer_pawn))
  (Variables|Default|SetparticleSystemLeft (Variables|/Game/Blueprints/Pawn/BP_VRPlayerPawn.BP_VRPlayerPawn_C|GetParticleSystemL _asbp_vrplayer_pawn))
  (Variables|Default|SetparticleSystemRight (Variables|/Game/Blueprints/Pawn/BP_VRPlayerPawn.BP_VRPlayerPawn_C|GetParticleSystemR _asbp_vrplayer_pawn))
  (Variables|Default|SetlastPosition (Transformation|GetWorldLocation (Variables|/Game/Blueprints/Pawn/BP_VRPlayerPawn.BP_VRPlayerPawn_C|GetCapsule _output_get))))

(event EventTick
  (params (DeltaSeconds :type Float%20%28single-precision%29))
  (bind _vrplayer (Variables|Default|GetVRPlayer))
  (Variables|Default|Setboost (* (+ (Math|Vector|GetForwardVector (Variables|/Game/Blueprints/Pawn/BP_VRPlayerPawn.BP_VRPlayerPawn_C|GetRight (Variables|Default|GetVRPlayer))) (Math|Vector|GetForwardVector (Variables|/Game/Blueprints/Pawn/BP_VRPlayerPawn.BP_VRPlayerPawn_C|GetLeft (Variables|Default|GetVRPlayer)))) (* (select (or (Variables|/Game/Blueprints/Pawn/BP_VRPlayerPawn.BP_VRPlayerPawn_C|GetboostLeft _vrplayer) (Variables|/Game/Blueprints/Pawn/BP_VRPlayerPawn.BP_VRPlayerPawn_C|GetboostRight _vrplayer)) (Variables|Default|GetboostPower) 0.0) (Utilities|Time|GetWorldDeltaSeconds)))))