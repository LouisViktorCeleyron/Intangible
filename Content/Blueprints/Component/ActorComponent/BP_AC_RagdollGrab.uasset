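; BP_AC_RagdollGrab is an unfinished actor component on the VR player pawn for grabbing physics-simulated meshes such as ragdolls.
; On BeginPlay it caches its owning BP_VRPlayerPawn, but the GrabBone event is empty.
; Disconnected logic selects the pawn's left or right physics handle by controller and grabs the mesh's bone at index zero, though the left-controller check is unwired.
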(event Custom|GrabBone
  (params (Controller :type Motion%20Controller%20Component%20Object%20Reference) (Mesh :type Skeletal%20Mesh%20Component%20Object%20Reference)))

(event EventBeginPlay
  (bind _asbp_vrplayer_pawn (Utilities|Casting|CastToBP_VRPlayerPawn (Components|GetOwner)))
  (Variables|Default|SetAs%20BP%20VRPlayer%20Pawn _asbp_vrplayer_pawn))