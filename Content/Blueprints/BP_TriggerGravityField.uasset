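; Trigger volume that marks a gravity field zone for the VR player pawn.
; The construction script derives the field's min and max Z from the collision component's bounds.
; On overlap, it flags BP_VRPlayerPawn as inside the field and passes it those Z limits, then clears the flag on exit.
; Both overlap events also print debug strings.
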(event OnComponentBeginOverlap(CollisionComponent)
  (params (OverlappedComponent :type Primitive%20Component%20Object%20Reference) (OtherActor :type Actor%20Object%20Reference) (OtherComp :type Primitive%20Component%20Object%20Reference) (OtherBodyIndex :type Integer) (bFromSweep :type Boolean) (SweepResult :type Hit%20Result%20Structure%20%28by%20ref%29))
  (bind _asbp_vrplayer_pawn (Utilities|Casting|CastToBP_VRPlayerPawn OtherActor))
  (Development|PrintString "IM IN BITCHES" true true "(R=0.000000,G=0.660000,B=1.000000,A=1.000000)" 5.0)
  (Variables|/Game/Blueprints/Pawn/BP_VRPlayerPawn.BP_VRPlayerPawn_C|SetisInGravityField _asbp_vrplayer_pawn true)
  (Variables|/Game/Blueprints/Pawn/BP_VRPlayerPawn.BP_VRPlayerPawn_C|SetminZGravityField _asbp_vrplayer_pawn (Variables|Default|GetminZ))
  (Variables|/Game/Blueprints/Pawn/BP_VRPlayerPawn.BP_VRPlayerPawn_C|SetmaxZGravityField _asbp_vrplayer_pawn (Variables|Default|GetmaxZ)))

(event OnComponentEndOverlap(CollisionComponent)
  (params (OverlappedComponent :type Primitive%20Component%20Object%20Reference) (OtherActor :type Actor%20Object%20Reference) (OtherComp :type Primitive%20Component%20Object%20Reference) (OtherBodyIndex :type Integer))
  (bind _asbp_vrplayer_pawn (Utilities|Casting|CastToBP_VRPlayerPawn OtherActor))
  (Development|PrintString "IM OUT BITCHES" true true "(R=0.000000,G=0.660000,B=1.000000,A=1.000000)" 5.0)
  (Variables|/Game/Blueprints/Pawn/BP_VRPlayerPawn.BP_VRPlayerPawn_C|SetisInGravityField _asbp_vrplayer_pawn false))

(event EventBeginPlay)

(event Collision|EventActorBeginOverlap
  (params (OtherActor :type Actor%20Object%20Reference)))

(event EventTick
  (params (DeltaSeconds :type Float%20%28single-precision%29)))

(fn ConstructionScript
  (bind _collisioncomponent (Variables|Default|GetCollisionComponent))
  (bind (_origin _boxextent) (Collision|GetComponentBounds _collisioncomponent))
  (Variables|Default|SetminZ (- (.z _origin) (.z _boxextent)))
  (Variables|Default|SetmaxZ (+ (.z _origin) (.z _boxextent))))